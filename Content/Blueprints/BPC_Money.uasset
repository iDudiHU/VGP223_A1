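; BPC_Money is a component that holds the player's money balance and handles earning and spending it.
; On BeginPlay it binds to the passenger-delivered event of the level's BP_PlatformManager, adding a fixed reward per delivery.
; TryBuy deducts a cost only when funds suffice and returns whether it succeeded.
; Both income and successful purchases broadcast OnMoneyChanged with the new balance.
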(event Custom|OnPassengerDelivered
  (CallFunction|AddMoney 3000)
  (Default|CallOnMoneyChanged (Variables|Default|GetMoney)))

(event EventBeginPlay
  (bind _returnvalue (Actor|GetActorOfClass "/Game/Blueprints/Managers/BP_PlatformManager.BP_PlatformManager_C"))
  (EventDispatchers|BindEventtoOnPassengerDelivered _returnvalue (delegate Custom|OnPassengerDelivered)))

(event EventTick
  (params (DeltaSeconds :type Float%20%28single-precision%29)))

(fn TryBuy
  (params (Cost :type Integer))
  (if (>= (Variables|Default|GetMoney) Cost)
    (CallFunction|SpendMoney Cost)
    (Default|CallOnMoneyChanged (Variables|Default|GetMoney))
    (return true)
    (else
      (return false))))

(fn SpendMoney
  (params (Cost :type Integer))
  (Variables|Default|SetMoney (- (Variables|Default|GetMoney) Cost)))

(fn AddMoney
  (params (Ammount :type Integer))
  (Variables|Default|SetMoney (+ Ammount (Variables|Default|GetMoney))))