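; B_LanderTaxi is a player-controlled lander taxi steered with main, left and right thrusters.
; BeginPlay adds the IMC_Taxi Enhanced Input mapping context, and each thruster action toggles a pair of thrust components on press and release.
; Main thruster audio plays while held, with its Speed parameter fed by the triggered time.
; Side thruster audio fades in and out, with left input driving the right-side audio and vice versa.
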(event Input|EnhancedActionEvents|EnhancedInputActionIA_Main_Thruster
  (params (ActionValue :type Boolean) (ElapsedSeconds :type Float%20%28double-precision%29) (TriggeredSeconds :type Float%20%28double-precision%29) (InputAction :type Input%20Action%20Object%20Reference :default "/Game/Input/IA_Main_Thruster.IA_Main_Thruster"))
  (bind _mainthruster (Variables|Default|GetMainThruster))
  (bind _mainthrusteraudio (Variables|Default|GetMainThrusterAudio))
  (:Triggered
    (Audio|Parameter|SetFloatParameter (Variables|Default|GetMainThrusterAudio) "Speed" TriggeredSeconds :!class /Script/Engine.AudioComponent))
  (:Started
    (Components|Activation|SetActive _mainthruster true false)
    (Audio|Components|Audio|Play _mainthrusteraudio 0.0))
  (:Completed
    (Components|Activation|SetActive _mainthruster false false)
    (Audio|Components|Audio|Stop _mainthrusteraudio)))

(event Input|EnhancedActionEvents|EnhancedInputActionIA_Left_Thruster
  (params (ActionValue :type Boolean) (ElapsedSeconds :type Float%20%28double-precision%29) (TriggeredSeconds :type Float%20%28double-precision%29) (InputAction :type Input%20Action%20Object%20Reference :default "/Game/Input/IA_Left_Thruster.IA_Left_Thruster"))
  (bind _leftthrust (Variables|Default|GetLeftThrust))
  (bind _rightthrusteraudio (Variables|Default|GetRightThrusterAudio))
  (:Started
    (Components|Activation|SetActive _leftthrust true false)
    (Audio|Components|Audio|FadeIn _rightthrusteraudio 0.1 1.0 0.0 "Logarithmic" :!class /Script/Engine.AudioComponent))
  (:Completed
    (Components|Activation|SetActive _leftthrust false false)
    (Audio|Components|Audio|FadeOut _rightthrusteraudio 0.1 0.0 "Linear" :!class /Script/Engine.AudioComponent)))

(event Input|EnhancedActionEvents|EnhancedInputActionIA_Right_Thruster
  (params (ActionValue :type Boolean) (ElapsedSeconds :type Float%20%28double-precision%29) (TriggeredSeconds :type Float%20%28double-precision%29) (InputAction :type Input%20Action%20Object%20Reference :default "/Game/Input/IA_Right_Thruster.IA_Right_Thruster"))
  (bind _leftthrusteraudio (Variables|Default|GetLeftThrusterAudio))
  (bind _rightthruster (Variables|Default|GetRightThruster))
  (:Started
    (Components|Activation|SetActive _rightthruster true false)
    (Audio|Components|Audio|FadeIn _leftthrusteraudio 0.1 1.0 0.0 "Logarithmic" :!class /Script/Engine.AudioComponent))
  (:Completed
    (Components|Activation|SetActive _rightthruster false false)
    (Audio|Components|Audio|FadeOut _leftthrusteraudio 0.1 0.0 "Linear" :!class /Script/Engine.AudioComponent)))

(event EventBeginPlay
  (bind _asplayer_controller (Utilities|Casting|CastToPlayerController (Pawn|GetController)))
  ;[1 0.9425 0] Don't forget to select your Mapping Context!
  (Input|AddMappingContext (PlayerController|LocalPlayerSubsystems|GetEnhancedInputLocalPlayerSubsystem _asplayer_controller) "/Game/Input/IMC_Taxi.IMC_Taxi" 0 "(bIgnoreAllPressedKeysUntilRelease=True,bForceImmediately=False)"))

(fn ConstructionScript)