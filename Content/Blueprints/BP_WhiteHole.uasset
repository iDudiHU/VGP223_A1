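; White hole actor that pulls a lander taxi toward the center of its sphere of influence, despite its name.
; Sphere overlaps set or clear the B_LanderTaxi target, and Tick pulls it while valid.
; The pull offsets TaxiVisual in world space without sweep or physics, scaled by frame time and Force, fading to half strength with distance.
; Debug drawing and alternative local-offset and AddForce approaches remain disconnected.
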(event OnComponentBeginOverlap(SphereOfInfluence)
  (params (OverlappedComponent :type Primitive%20Component%20Object%20Reference) (OtherActor :type Actor%20Object%20Reference) (OtherComp :type Primitive%20Component%20Object%20Reference) (OtherBodyIndex :type Integer) (bFromSweep :type Boolean) (SweepResult :type Hit%20Result%20Structure%20%28by%20ref%29))
  (bind _asb_lander_taxi (Utilities|Casting|CastToB_LanderTaxi OtherActor))
  (Variables|Default|SetTarget _asb_lander_taxi))

(event OnComponentEndOverlap(SphereOfInfluence)
  (params (OverlappedComponent :type Primitive%20Component%20Object%20Reference) (OtherActor :type Actor%20Object%20Reference) (OtherComp :type Primitive%20Component%20Object%20Reference) (OtherBodyIndex :type Integer))
  (Utilities|Casting|CastToB_LanderTaxi OtherActor)
  (Variables|Default|SetTarget 0))

(event Custom|PullTowardsCenter
  (bind _target (Variables|Default|GetTarget))
  (bind _sphereofinfluence (Variables|Default|GetSphereOfInfluence))
  (bind _returnvalue (Transformation|GetWorldLocation _sphereofinfluence))
  (bind _taxi_visual (Variables|/Game/Blueprints/B_LanderTaxi.B_LanderTaxi_C|GetTaxi_Visual _target))
  (bind _returnvalue_2 (Transformation|GetWorldLocation _taxi_visual))
  (bind _returnvalue_3 (- _returnvalue_2 _returnvalue))
  (bind _returnvalue_4 (* _returnvalue_3 -1))
  (Transformation|AddWorldOffset _taxi_visual (* (Math|Vector|Normalize _returnvalue_4) (Utilities|Time|GetWorldDeltaSeconds) (* (Math|Float|MapRangeClamped (Math|Vector|VectorLength _returnvalue_4) 0.0 3e+03 1.0 0.5) (Variables|Default|GetForce))) false false))

(event EventBeginPlay)

(event Collision|EventActorBeginOverlap
  (params (OtherActor :type Actor%20Object%20Reference)))

(event EventTick
  (params (DeltaSeconds :type Float%20%28single-precision%29))
  (Variables|Default|GetTarget
    (:then
      (CallFunction|PullTowardsCenter))
    (:else)))

(fn ConstructionScript)