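; BP_Health_Pickup is a pickup that restores health to the lander taxi (B_LanderTaxi) on contact.
; Its box overlap accepts only that class and heals by sending HealAmmount as negative damage through ApplyDamage, reusing the damage path.
; It then deactivates its Niagara effect, plays a sound, activates the Pickup component and destroys itself after a short delay.
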(event OnComponentBeginOverlap(Box)
  (params (OverlappedComponent :type Primitive%20Component%20Object%20Reference) (OtherActor :type Actor%20Object%20Reference) (OtherComp :type Primitive%20Component%20Object%20Reference) (OtherBodyIndex :type Integer) (bFromSweep :type Boolean) (SweepResult :type Hit%20Result%20Structure%20%28by%20ref%29))
  (bind _asb_lander_taxi (Utilities|Casting|CastToB_LanderTaxi OtherActor))
  (Game|Damage|ApplyDamage _asb_lander_taxi (* (Variables|Default|GetHealAmmount) -1.0) 0 0)
  (Components|Activation|Deactivate (Variables|Default|GetNiagara))
  (Audio|PlaySoundatLocation "/Game/Sound/Sci-Fi_Sounds/Shield/shield_special.shield_special" "0, 0, 0" "0, 0, 0" 1.0 1.0 0.0 0 0 0 0)
  (Components|Activation|Activate (Variables|Default|GetPickup) false)
  (Utilities|FlowControl|Delay 0.6)
  (Actor|DestroyActor))

(event EventBeginPlay)

(event Collision|EventActorBeginOverlap
  (params (OtherActor :type Actor%20Object%20Reference)))

(event EventTick
  (params (DeltaSeconds :type Float%20%28single-precision%29)))

(fn ConstructionScript)