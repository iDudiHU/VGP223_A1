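; Shop actor where the player's lander taxi can open a shop menu while inside a trigger box.
; Box overlap stores the taxi, shows a text prompt and binds to its ship-changed event to update a display ship mesh; leaving hides the prompt.
; Interact blends the view to the shop camera, calls OpenShop on the taxi, then pauses the game after a short delay.
; The Heal function is an empty stub.
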(event OnComponentBeginOverlap(Box)
  (params (OverlappedComponent :type Primitive%20Component%20Object%20Reference) (OtherActor :type Actor%20Object%20Reference) (OtherComp :type Primitive%20Component%20Object%20Reference) (OtherBodyIndex :type Integer) (bFromSweep :type Boolean) (SweepResult :type Hit%20Result%20Structure%20%28by%20ref%29))
  (bind _asb_lander_taxi (Utilities|Casting|CastToB_LanderTaxi OtherActor))
  (bind _output_get (Variables|Default|SetPlayer _asb_lander_taxi))
  (CallFunction|Interactible _output_get)
  (EventDispatchers|BindEventtoOnShipChanged _output_get (delegate Custom|OnShipChanged)))

(event OnComponentEndOverlap(Box)
  (params (OverlappedComponent :type Primitive%20Component%20Object%20Reference) (OtherActor :type Actor%20Object%20Reference) (OtherComp :type Primitive%20Component%20Object%20Reference) (OtherBodyIndex :type Integer))
  (CallFunction|Unintaractible)
  (Variables|Default|SetPlayer 0))

(event Custom|OnShipChanged
  (params (ShipVisual :type Static%20Mesh%20Object%20Reference))
  (Components|StaticMesh|SetStaticMesh (Variables|Default|GetShipVisual) ShipVisual))

(event EventBeginPlay)

(event Collision|EventActorBeginOverlap
  (params (OtherActor :type Actor%20Object%20Reference)))

(event EventTick
  (params (DeltaSeconds :type Float%20%28single-precision%29)))

(event EventInteract
  (if (Variables|Default|GetPlayer_Can_Interact)
    (Game|Player|SetViewTargetwithBlend (Game|GetPlayerController 0) (Variables|Default|GetCamera) 0.7 "VTBlend_Cubic" 0.0 false)
    (Default|OpenShop (Variables|Default|GetPlayer))
    (Utilities|FlowControl|Delay 1.0)
    (Game|SetGamePaused true)))

(fn ConstructionScript)

(fn Heal)

(fn Interactible
  (params (Other :type Actor%20Object%20Reference))
  (Variables|Default|SetPlayer_Can_Interact true)
  (Rendering|SetVisibility (Variables|Default|GetTextRender) true false))

(fn Unintaractible
  (Variables|Default|SetPlayer_Can_Interact false)
  (Rendering|SetVisibility (Variables|Default|GetTextRender) false false))