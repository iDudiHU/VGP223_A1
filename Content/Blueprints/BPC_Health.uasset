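; BPC_Health is a component that tracks its owner's health, starting at MaxHealth and responding to the owner's any-damage event.
; Positive damage is ignored while immune; zero or negative damage always applies, so negative values heal.
; Each applied change clamps health to a fixed 0–100 range, not MaxHealth, and broadcasts OnHealthChanged, plus OnHealthDepleted at zero.
; It also starts one second of immunity, even after healing, cleared by a ResetImmune timer.
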(event Custom|OnTakeAnyDamage_Event
  (params (DamagedActor :type Actor%20Object%20Reference) (Damage :type Float%20%28single-precision%29) (DamageType :type Damage%20Type%20Object%20Reference) (InstigatedBy :type Controller%20Object%20Reference) (DamageCauser :type Actor%20Object%20Reference))
  (if (<= Damage 0.0)
    (bind _output_get (Variables|Default|SetCurrentHealth (Math|Float|Clamp(Float) (- (Variables|Default|GetCurrentHealth) Damage) 0.0 1e+02) :!label _label))
    (Default|CallOnHealthChanged _output_get (Variables|Default|GetMaxHealth))
    (Variables|Default|SetImmune true)
    (Utilities|Time|SetTimerbyFunctionName 0 "ResetImmune" 1.0)
    (if (<= (Variables|Default|GetCurrentHealth) 0.0)
      (Default|CallOnHealthDepleted))
    (elif (not (Variables|Default|GetImmune))
      (goto _label))))

(event EventBeginPlay
  (Variables|Default|SetCurrentHealth (Variables|Default|GetMaxHealth))
  (EventDispatchers|AssignOnTakeAnyDamage (Components|GetOwner) (delegate Custom|OnTakeAnyDamage_Event)))

(fn ResetImmune
  (Variables|Default|SetImmune false))