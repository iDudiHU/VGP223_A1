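; B_Mine is a moving mine that explodes when a B_LanderTaxi overlaps its sphere.
; The construction script feeds points A and B and Duration into InterpToMovement as a relative path.
; A looping timer with a randomly chosen interval plays an attenuated alarm sound at the mesh.
; A one-shot overlap damages the taxi, shoves it away, triggers particles, camera shake and explosion sound, then destroys the mine after a short delay.
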(event OnComponentBeginOverlap(Sphere)
  (params (OverlappedComponent :type Primitive%20Component%20Object%20Reference) (OtherActor :type Actor%20Object%20Reference) (OtherComp :type Primitive%20Component%20Object%20Reference) (OtherBodyIndex :type Integer) (bFromSweep :type Boolean) (SweepResult :type Hit%20Result%20Structure%20%28by%20ref%29))
  (bind _returnvalue (Transformation|GetActorLocation))
  (bind _asb_lander_taxi (Utilities|Casting|CastToB_LanderTaxi OtherActor))
  (Utilities|FlowControl|DoOnce false
    (:Completed
      (Game|Damage|ApplyDamage _asb_lander_taxi 25.0 0 0)
      (Physics|AddForce (Variables|/Game/Blueprints/B_LanderTaxi.B_LanderTaxi_C|GetTaxi_Visual _asb_lander_taxi) (* (Math|Vector|GetUnitDirection(Vector) (Transformation|GetWorldLocation (Variables|/Script/Engine.Actor|GetRootComponent _asb_lander_taxi)) (Transformation|GetActorLocation)) -1e+04) "None" false)
      (Components|Activation|Activate (Variables|Default|GetParticleSystem) true)
      (Camera|PlayWorldCameraShake "/Game/Blueprints/Camera/BP_Camera_Shake.BP_Camera_Shake_C" _returnvalue 0.0 1e+07 0.0)
      (Audio|PlaySoundatLocation "/Game/Sound/Sci-Fi_Sounds/Explosion/explosion_med_010.explosion_med_010" _returnvalue "0, 0, 0" 1.0 1.0 0.0 "/Game/Audio/Attenuations/SA_Mine.SA_Mine" 0 0 0)
      (Components|Activation|Deactivate (Variables|Default|GetStaticMesh))
      (Utilities|FlowControl|Delay 0.3)
      (Actor|DestroyActor))))

(event EventBeginPlay
  (Utilities|Time|SetTimerbyFunctionName 0 "PlayMineSFX" (Math|Random|RandomFloatinRange 2.0 4.0) true))

(fn ConstructionScript
  (bind _interptomovement (Variables|Default|GetInterpToMovement))
  (Variables|/Script/Engine.InterpToMovementComponent|SetControlPoints _interptomovement (Utilities|Array|MakeArray (Utilities|Struct|MakeInterpControlPoint (Variables|Default|GetA) true) (Utilities|Struct|MakeInterpControlPoint (Variables|Default|GetB) true)))
  (Variables|/Script/Engine.InterpToMovementComponent|SetDuration _interptomovement (Variables|Default|GetDuration)))

(fn PlayMineSFX
  (Audio|PlaySoundatLocation "/Game/Sound/Sci-Fi_Sounds/Bonus/bonus_alarm_003.bonus_alarm_003" (Transformation|GetWorldLocation (Variables|Default|GetStaticMesh)) "0, 0, 0" 1.4 1.0 0.0 "/Game/Audio/Attenuations/SA_Mine.SA_Mine" 0 0 0))