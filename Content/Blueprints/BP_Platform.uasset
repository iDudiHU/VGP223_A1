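; BP_Platform is a landing pad where the player's B_LanderTaxi picks up and delivers passengers.
; A box overlap marks the taxi as docking, and Tick treats it as docked once its Speed drops to zero.
; Docking then triggers a pickup or, on the target pad, a delivery, both reported to BP_PlatformManager.
; AddPassenger and SetTargetPlatform set the pad's state and show FXSignaler with a pickup or target material.
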(event OnComponentEndOverlap(BoxCollider)
  (params (OverlappedComponent :type Primitive%20Component%20Object%20Reference) (OtherActor :type Actor%20Object%20Reference) (OtherComp :type Primitive%20Component%20Object%20Reference) (OtherBodyIndex :type Integer))
  (Utilities|Casting|CastToB_LanderTaxi OtherActor)
  (Variables|Default|SetPlayerDocked false)
  (Variables|Default|SetPlayerDocking false))

(event OnComponentBeginOverlap(BoxCollider)
  (params (OverlappedComponent :type Primitive%20Component%20Object%20Reference) (OtherActor :type Actor%20Object%20Reference) (OtherComp :type Primitive%20Component%20Object%20Reference) (OtherBodyIndex :type Integer) (bFromSweep :type Boolean) (SweepResult :type Hit%20Result%20Structure%20%28by%20ref%29))
  (bind _asb_lander_taxi (Utilities|Casting|CastToB_LanderTaxi OtherActor))
  (Variables|Default|SetPlayerDocking true)
  (bind _output_get (Variables|Default|SetPlayer _asb_lander_taxi)))

(event EventBeginPlay
  (bind _returnvalue (Actor|GetActorOfClass "/Game/Blueprints/Managers/BP_PlatformManager.BP_PlatformManager_C"))
  (Variables|Default|SetManager _returnvalue)
  (Rendering|SetVisibility (Variables|Default|GetFX_Signaler) false false))

(event EventTick
  (params (DeltaSeconds :type Float%20%28single-precision%29))
  (if (Variables|Default|GetPlayerDocking)
    (bind _output_get (Variables|Default|SetPlayerDocked (<= (Variables|/Game/Blueprints/B_LanderTaxi.B_LanderTaxi_C|GetSpeed (stale OnComponentBeginOverlap(BoxCollider) _output_get)) 0.0)))
    (if _output_get
      (if (Variables|Default|GetHasPassenger)
        (Development|PrintString "Player Picked Up Passenger")
        (CallFunction|PickupPassenger)
        (Default|PickUpPassenger (Variables|Default|GetManager))
        (elif (Variables|Default|GetIsCurrentTarget)
          (Development|PrintString "Passenger delivered")
          (Default|DeliverPassenger (Variables|Default|GetManager))
          (Variables|Default|SetIsCurrentTarget false)
          (Rendering|SetVisibility (Variables|Default|GetFX_Signaler) false false))))))

(fn ConstructionScript)

(fn AddPassenger
  (bind _fx_signaler (Variables|Default|GetFX_Signaler))
  (Variables|Default|SetHasPassenger true)
  (Variables|Default|SetIsCurrentTarget false)
  (Rendering|Material|SetMaterial _fx_signaler 0 (Variables|Default|GetPickup))
  (Rendering|SetVisibility _fx_signaler true false))

(fn PickupPassenger
  (Rendering|SetVisibility (Variables|Default|GetFX_Signaler) false false)
  (Variables|Default|SetHasPassenger false)
  (Audio|PlaySound2D "/Game/Sound/Sci-Fi_Sounds/Mechanical/mechanical_cargo_load_003.mechanical_cargo_load_003" 0.6 1.0 0.0 0 0))

(fn SetTargetPlatform
  (bind _fx_signaler (Variables|Default|GetFX_Signaler))
  (Variables|Default|SetIsCurrentTarget true)
  (Rendering|Material|SetMaterial _fx_signaler 0 (Variables|Default|GetTarget))
  (Rendering|SetVisibility _fx_signaler true false))