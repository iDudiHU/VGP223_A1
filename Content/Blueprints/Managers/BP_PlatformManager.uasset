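; BP_PlatformManager is a manager that tracks the level's BP_Platform actors, apparently to distribute passengers among them.
; On BeginPlay it gathers every BP_Platform into the Platforms array.
; AssignPassengers is unfinished: it picks and casts a random platform but assigns nothing, and its loop never runs because its equality condition contradicts the preceding less-than check on AllocatedPassengers and MaxPassengers.
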(event EventBeginPlay
  (bind _outactors (Actor|GetAllActorsOfClass "/Game/Blueprints/BP_Platform.BP_Platform_C"))
  (Variables|Default|SetPlatforms _outactors))

(event Collision|EventActorBeginOverlap
  (params (OtherActor :type Actor%20Object%20Reference)))

(event EventTick
  (params (DeltaSeconds :type Float%20%28single-precision%29)))

(fn ConstructionScript)

(fn AssignPassengers
  (bind _platforms (Variables|Default|GetPlatforms))
  (if (< (Variables|Default|GetAllocatedPassengers) (Variables|Default|GetMaxPassengers))
    (while (== (Variables|Default|GetAllocatedPassengers) (Variables|Default|GetMaxPassengers))
      (Utilities|Casting|CastToBP_Platform (Utilities|Array|Get(acopy) _platforms (Math|Random|RandomIntegerinRange 0 (Utilities|Array|LastIndex _platforms)))))))